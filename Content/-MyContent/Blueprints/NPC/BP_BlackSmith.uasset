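; BP_BlackSmith is the blacksmith NPC, which opens a shop-style interaction widget when the player comes near.
; Overlapping the interaction zone as player character 0 shows WB_BlackSmith and the cursor; any end overlap removes both.
; SetUpLocal, not called here, sets the name "Forgerer" through a server event, and its OnRep fills the overhead WB_PlayerName widget.
; The OnRep's retry timer targets OnRep_CustomPlayerName, a function absent here.
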(event OnComponentBeginOverlap(InteractionZone)
  (params (OverlappedComponent :type Primitive%20Component%20Object%20Reference) (OtherActor :type Actor%20Object%20Reference) (OtherComp :type Primitive%20Component%20Object%20Reference) (OtherBodyIndex :type Integer) (bFromSweep :type Boolean) (SweepResult :type Hit%20Result%20Structure%20%28by%20ref%29))
  (if (== (Game|GetPlayerCharacter 0) OtherActor)
    (bind _returnvalue (UserInterface|CreateWidget "/Game/-MyContent/UI/NPC/WB_BlackSmith.WB_BlackSmith_C"))
    (bind _output_get (Variables|Default|SetWidgetInteraction _returnvalue))
    (UserInterface|Viewport|AddtoViewport _output_get 0)
    (Variables|/Script/Engine.PlayerController|SetbShowMouseCursor (Game|GetPlayerController 0) true)))

(event OnComponentEndOverlap(InteractionZone)
  (params (OverlappedComponent :type Primitive%20Component%20Object%20Reference) (OtherActor :type Actor%20Object%20Reference) (OtherComp :type Primitive%20Component%20Object%20Reference) (OtherBodyIndex :type Integer))
  (Class|GameViewportSubsystem|RemoveWidget (|GameViewportSubsystem) (Variables|Default|GetWidgetInteraction))
  (Variables|/Script/Engine.PlayerController|SetbShowMouseCursor (Game|GetPlayerController 0) false))

(event Custom|SetNPCName%20on%20Server
  (params (CustomPlayerName :type Text))
  ;[1 1 1] Set NPC Name
  (Variables|Default|SetNPCName CustomPlayerName))

(fn ConstructionScript)

(fn OnRepCustomNPCName
  (bind _w_npcname (Variables|Default|GetW_NPCName))
  (bind _returnvalue (UserInterface|GetWidget _w_npcname))
  (Utilities|IsValid _returnvalue
    (:Is%20Valid
      (bind _aswb_player_name (Utilities|Casting|CastToWB_PlayerName _returnvalue))
      (Default|SetPlayerName _aswb_player_name (Variables|Default|GetNPCName))
      (Development|SetHiddeninGame (Variables|Default|GetW_NPCName) false false))
    (:Is%20Not%20Valid
      (Utilities|Time|SetTimerbyFunctionName 0 "OnRep_CustomPlayerName" 0.1))))

(fn SetUpLocal
  (Utilities|Casting|CastToGI_TwinDungeons (Game|GetGameInstance))
  (CallFunction|SetNPCNameonServer "Forgerer"))