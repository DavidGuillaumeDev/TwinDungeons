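; BP_SelectionCharacter is the preview character for class selection, cycling through the available character meshes.
; Each ChangeCharacter call advances an index through the Characters array, wrapping to the start, and applies that skeletal mesh to its Mesh component.
; It then writes the index to ClassSelectedIndex on the GI_TwinDungeons game instance, so the selection is held outside the actor.
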(event Custom|Change%20Character
  (if (< (Variables|Default|GetCurrentCharacterIndex) (- (Utilities|Array|Length (Variables|Default|GetCharacters)) 1))
    (Math|Integer|IncrementInt (Variables|Default|GetCurrentCharacterIndex)
      (:%20%20
        _))
    (else
      (Variables|Default|SetCurrentCharacterIndex 0)))
  (Components|SkeletalMesh|SetSkeletalMeshAsset (Variables|Default|GetMesh) (Utilities|Array|Get(acopy) (Variables|Default|GetCharacters) (Variables|Default|GetCurrentCharacterIndex)))
  (bind _asgi_twin_dungeons (Utilities|Casting|CastToGI_TwinDungeons (Game|GetGameInstance)))
  (Variables|/Game/-MyContent/Blueprints/GI_TwinDungeons.GI_TwinDungeons_C|SetClassSelectedIndex _asgi_twin_dungeons (Variables|Default|GetCurrentCharacterIndex)))

(fn ConstructionScript)