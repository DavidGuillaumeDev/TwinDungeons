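; PC_MainMenu is the player controller Blueprint that sets up the main menu UI.
; On BeginPlay, for the local controller only, it creates the main menu, create server, server browser and load server widgets and stores a reference to each.
; Only the main menu widget is added to the viewport; the other three are created up front but not displayed here.
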(event EventBeginPlay
  (if (Pawn|IsLocalPlayerController)
    (bind _returnvalue (UserInterface|CreateWidget "/Game/-MyContent/UI/MENU/WB_MainMenu.WB_MainMenu_C"))
    (bind _output_get (Variables|Default|SetWB_MainMenu _returnvalue))
    (UserInterface|Viewport|AddtoViewport _output_get 0)
    (bind _returnvalue_2 (UserInterface|CreateWidget "/Game/-MyContent/UI/MENU/WB_CreateServer.WB_CreateServer_C"))
    (Variables|Default|SetWB_CreateServer _returnvalue_2)
    (bind _returnvalue_3 (UserInterface|CreateWidget "/Game/-MyContent/UI/MENU/WB_ServerBrowser.WB_ServerBrowser_C"))
    (Variables|Default|SetWB_ServerBrowser _returnvalue_3)
    (bind _returnvalue_4 (UserInterface|CreateWidget "/Game/-MyContent/UI/MENU/WB_LoadServer.WB_LoadServer_C"))
    (Variables|Default|SetWB_LoadServer _returnvalue_4)))

(fn ConstructionScript)