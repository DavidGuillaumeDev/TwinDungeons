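; PC_Game is a player controller that toggles a player list widget with the Tab key.
; On the local controller, a FlipFlop alternates between creating the widget, adding it to the viewport with the mouse cursor shown, and removing it with the cursor hidden.
; The stored widget reference is validity-checked before each step and cleared on removal, so each opening constructs a fresh widget.
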(event Input|KeyboardEvents|Tab
  (params (Key :type Key%20Structure :default "None"))
  (:Pressed
    (if (Pawn|IsLocalPlayerController)
      (Utilities|FlowControl|FlipFlop
        (:A
          (Variables|Default|GetWB_PlayerList
            (:then)
            (:else
              (bind _returnvalue (Game|ConstructObjectfromClass self "/Game/-MyContent/UI/MENU/WB_PlayerList.WB_PlayerList_C"))
              (bind _output_get (Variables|Default|SetWB_PlayerList _returnvalue))
              (UserInterface|Viewport|AddtoViewport _output_get 0)
              (Variables|Default|SetbShowMouseCursor true))))
        (:B
          (bind _wb_playerlist (Variables|Default|GetWB_PlayerList)
            (:then
              (Widget|RemovefromParent _wb_playerlist)
              (Variables|Default|SetWB_PlayerList 0)
              (Variables|Default|SetbShowMouseCursor false))
            (:else)))))))

(fn ConstructionScript)