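; Interactable portal actor that moves the player to another level.
; An overlap box shows a prompt widget while the player character is inside and hides it on exit.
; Interact opens the referenced level unless the actor is hidden, and a PortalVisibility event unhides the portal.
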(event OnComponentBeginOverlap(Box)
  (params (OverlappedComponent :type Primitive%20Component%20Object%20Reference) (OtherActor :type Actor%20Object%20Reference) (OtherComp :type Primitive%20Component%20Object%20Reference) (OtherBodyIndex :type Integer) (bFromSweep :type Boolean) (SweepResult :type Hit%20Result%20Structure%20%28by%20ref%29))
  (if (== (Game|GetPlayerCharacter 0) OtherActor)
    (Rendering|SetVisibility (Variables|Default|GetWidget) true false)))

(event OnComponentEndOverlap(Box)
  (params (OverlappedComponent :type Primitive%20Component%20Object%20Reference) (OtherActor :type Actor%20Object%20Reference) (OtherComp :type Primitive%20Component%20Object%20Reference) (OtherBodyIndex :type Integer))
  (Rendering|SetVisibility (Variables|Default|GetWidget) false false))

(event Custom|Portal%20Visibility
  (Rendering|SetActorHiddenInGame false))

(event EventInteract
  (if (not (Variables|Rendering|GetbHidden))
    (Game|OpenLevel(byObjectReference) (Variables|Default|GetLevel))))

(fn ConstructionScript)