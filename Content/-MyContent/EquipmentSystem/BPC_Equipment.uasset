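; Equipment component that toggles an equipment panel for its owning third-person character and keeps a list of weapon slots.
; The inventory input creates WB_Equipment, shows the cursor, switches to game-and-UI input and freezes the character by setting movement mode to None.
; Pressing it again removes the widget and restores game-only input and walking.
; AddWeapon appends an item to WeaponSlots.
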(event Input|EnhancedActionEvents|EnhancedInputActionIA_Inventory
  (params (ActionValue :type Boolean) (ElapsedSeconds :type Float%20%28double-precision%29) (TriggeredSeconds :type Float%20%28double-precision%29) (InputAction :type Input%20Action%20Object%20Reference :default "/Game/ThirdPerson/Input/Actions/IA_Inventory.IA_Inventory"))
  (bind _returnvalue (Game|GetPlayerController 0))
  ;[1 1 1] Equipment Inventory
  (:Started
    (if (not (Variables|Default|GetisPanelOpened?))
      (Variables|Default|SetisPanelOpened? true)
      (bind _returnvalue_2 (UserInterface|CreateWidget "/Game/-MyContent/UI/EQUIPMENT/WB_Equipment.WB_Equipment_C"))
      (bind _output_get (Variables|Default|SetEquipmentWidget _returnvalue_2))
      (UserInterface|Viewport|AddtoViewport _output_get 0)
      (Variables|/Script/Engine.PlayerController|SetbShowMouseCursor _returnvalue true)
      (Input|SetInputModeGameandUI _returnvalue (Variables|Default|GetEquipmentWidget) "DoNotLock" true false)
      (bind _asbp_third_person_character (Utilities|Casting|CastToBP_ThirdPersonCharacter (Components|GetOwner)))
      (Pawn|Components|CharacterMovement|SetMovementMode (Variables|/Script/Engine.Character|GetCharacterMovement _asbp_third_person_character) "MOVE_None" 0)
      (else
        (Variables|Default|SetisPanelOpened? false)
        (bind _equipmentwidget (Variables|Default|GetEquipmentWidget)
          (:then
            (Widget|RemovefromParent _equipmentwidget)
            (Variables|Default|SetEquipmentWidget 0)
            (Variables|/Script/Engine.PlayerController|SetbShowMouseCursor _returnvalue false)
            (Input|SetInputModeGameOnly _returnvalue false)
            (bind _asbp_third_person_character_2 (Utilities|Casting|CastToBP_ThirdPersonCharacter (Components|GetOwner)))
            (Pawn|Components|CharacterMovement|SetMovementMode (Variables|/Script/Engine.Character|GetCharacterMovement _asbp_third_person_character_2) "MOVE_Walking" 0))
          (:else))))))

(fn AddWeapon
  (params (NewItem :type S%20Slots%20Structure%20%28by%20ref%29))
  (Utilities|Array|Add (Variables|Default|GetweaponSlots) NewItem))