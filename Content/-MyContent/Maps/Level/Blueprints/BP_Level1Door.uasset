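; BP_Level1Door is a sliding door that opens when the player character overlaps its Box or when the OpenDoor event is called.
; Each path plays a metal door sound and its own timeline, which drives the Door component's relative Z location.
; Timeline updates set a DoorOpen flag that blocks repeat overlap triggers; OpenDoor does not check it, and nothing here closes the door.
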(event OnComponentBeginOverlap(Box)
  (params (OverlappedComponent :type Primitive%20Component%20Object%20Reference) (OtherActor :type Actor%20Object%20Reference) (OtherComp :type Primitive%20Component%20Object%20Reference) (OtherBodyIndex :type Integer) (bFromSweep :type Boolean) (SweepResult :type Hit%20Result%20Structure%20%28by%20ref%29))
  ;[1 1 1] DoorMovement
  (if (== (Game|GetPlayerCharacter 0) OtherActor)
    (if (not (Variables|Default|GetDoorOpen?))
      (Audio|PlaySound2D "/Game/-MyContent/UI/SOUNDS/large-metal-sliding-door.large-metal-sliding-door" 1.0 1.0 0.0 0 0)
      (bind _door (Timeline|DoorOpen Play)
        (:Update
          (Transformation|SetRelativeLocation (Variables|Default|GetDoor) (Math|Vector|MakeVector 0.0 0.0 _door) false false)
          (Variables|Default|SetDoorOpen? true))))))

(event Custom|Open%20Door
  (Audio|PlaySound2D "/Game/-MyContent/UI/SOUNDS/large-metal-sliding-door.large-metal-sliding-door" 1.0 1.0 0.0 0 0)
  (bind _door (Timeline|Timeline Play)
    (:Update
      (Transformation|SetRelativeLocation (Variables|Default|GetDoor) (Math|Vector|MakeVector 0.0 0.0 _door) false false)
      (Variables|Default|SetDoorOpen? true))))

(fn ConstructionScript)