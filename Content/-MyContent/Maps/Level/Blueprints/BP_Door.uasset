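; BP_Door is a configurable door that opens by sliding along its vertical axis.
; BeginPlay applies the mesh, material and relative transform to the Door component, as the construction script is empty.
; OpenDoor plays a 2D sound and a timeline that scales ZHeight into the relative Z location, zeroing X and Y.
; Each timeline update also sets DoorOpen to true, and no closing logic exists.
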(event Custom|Open%20Door
  ;[1 1 1] Open Door
  (Audio|PlaySound2D (Variables|Default|GetSound) 1.0 1.0 0.0 0 0)
  (bind _door (Timeline|Timeline Play)
    (:Update
      (Transformation|SetRelativeLocation (Variables|Default|GetDoor) (Math|Vector|MakeVector 0.0 0.0 (* _door (Variables|Default|GetZHeight))) false false)
      (Variables|Default|SetDoorOpen? true))))

(event EventBeginPlay
  (bind _door (Variables|Default|GetDoor))
  ;[1 1 1] Parameters
  (Components|StaticMesh|SetStaticMesh _door (Variables|Default|GetMesh))
  (Rendering|Material|SetMaterial _door 0 (Variables|Default|GetMaterial))
  (Transformation|SetRelativeTransform _door (Variables|Default|GetNew%20Transform) false false))

(fn ConstructionScript)