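; Quest component that tracks the active quest's objectives and drives a quest HUD widget it creates on BeginPlay.
; EliminateEnnemy removes kills from a shared enemy array on a working quest copy, completing the objective when empty and optionally opening its BP_Door.
; OpenChest completes objectives whose target chest matches.
; Each completion updates the HUD and tallies completed objectives, clearing the quest and playing an animation once the tally reaches the objective count.
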(event Custom|Set%20Active%20Quest%20Text
  (Rendering|Components|TextRender|SetText (Variables|/Game/-MyContent/UI/HUD/WB_QuestHUD.WB_QuestHUD_C|GetActiveQuestText (Variables|Default|GetQuest%20HUD%20Widget)) (Utilities|Text|ToText(String) (.Name (Utilities|Struct|BreakS_Quest (Variables|Default|GetActiveQuest)))))
  (Default|ShowQuestPanel (Variables|Default|GetQuest%20HUD%20Widget))
  (Variables|Default|SetActiveQuestState (Variables|Default|GetActiveQuest)))

(event Custom|Set%20Objectives
  (Default|FillObjectives (Variables|Default|GetQuest%20HUD%20Widget) (.objectives (Variables|Default|GetActiveQuest))))

(event Custom|Eliminate%20Ennemy
  (params (Ennemy%20Eliminated :type Actor%20Object%20Reference))
  (bind _activequeststate (Variables|Default|GetActiveQuestState))
  (for (_array_element _array_index) (.objectives _activequeststate)
    (if (and (not (.Completed (Utilities|Struct|BreakS_QuestObjective _array_element))) (.IsEliminateEnnemyObjective (Utilities|Struct|BreakS_QuestObjective _array_element)))
      (if (!= (Utilities|Array|Length (Variables|Default|GetEnnemy%20Actors%20Array)) 0)
        _
        (else
          (bind _output_get (Variables|Default|SetEnnemy%20Actors%20Array (.ActorsToEliminate (Utilities|Struct|BreakS_QuestObjective _array_element))))))
      (Utilities|Array|RemoveItem _output_get Ennemy%20Eliminated)
      (|SetBy-RefVar _array_element (Utilities|Struct|MakeS_QuestObjective (.Name (Utilities|Struct|BreakS_QuestObjective _array_element)) false (Variables|Default|GetEnnemy%20Actors%20Array) (.ChestToOpen (Utilities|Struct|BreakS_QuestObjective _array_element)) (.IsEliminateEnnemyObjective (Utilities|Struct|BreakS_QuestObjective _array_element)) (.IsChestObjective (Utilities|Struct|BreakS_QuestObjective _array_element)) false 0))
      (if (== (Utilities|Array|Length (Variables|Default|GetEnnemy%20Actors%20Array)) 0)
        (|SetBy-RefVar _array_element (Utilities|Struct|MakeS_QuestObjective (.Name (Utilities|Struct|BreakS_QuestObjective _array_element)) true 0 (.ChestToOpen (Utilities|Struct|BreakS_QuestObjective _array_element)) (.IsEliminateEnnemyObjective (Utilities|Struct|BreakS_QuestObjective _array_element)) (.IsChestObjective (Utilities|Struct|BreakS_QuestObjective _array_element)) false 0))
        ;[1 1 1] Update the Total Quest Obj
        (|SetBy-RefVar (Utilities|Array|Get(acopy) (.objectives (Variables|Default|GetActiveQuest)) _array_index) (Utilities|Struct|MakeS_QuestObjective "" true 0 0 false false false 0))
        (Default|CompleteObjective (Variables|Default|GetQuest%20HUD%20Widget) _array_element)
        ;[1 1 1] Open Door
        (if (.IsDoorOpenning (Utilities|Struct|BreakS_QuestObjective _array_element))
          (bind _asbp_door (Utilities|Casting|CastToBP_Door (.DoortoOpen (Utilities|Struct|BreakS_QuestObjective _array_element))))
          (Default|OpenDoor _asbp_door))
        (CallFunction|ObjectiveCompleted)
        ;[1 1 1] Delete Obj Done
        (Utilities|Array|RemoveIndex (.objectives _activequeststate) _array_index)
        (Development|PrintString "Completed")))))

(event Custom|Open%20Chest
  (params (Chest :type Actor%20Object%20Reference))
  (for _array_element (.objectives (Variables|Default|GetActiveQuest))
    (if (and (.IsChestObjective (Utilities|Struct|BreakS_QuestObjective _array_element)) (== Chest (.ChestToOpen (Utilities|Struct|BreakS_QuestObjective _array_element))))
      (|SetBy-RefVar _array_element (Utilities|Struct|MakeS_QuestObjective (.Name (Utilities|Struct|BreakS_QuestObjective _array_element)) true (.ActorsToEliminate (Utilities|Struct|BreakS_QuestObjective _array_element)) 0 (.IsEliminateEnnemyObjective (Utilities|Struct|BreakS_QuestObjective _array_element)) (.IsChestObjective (Utilities|Struct|BreakS_QuestObjective _array_element)) false 0))
      (Default|CompleteObjective (Variables|Default|GetQuest%20HUD%20Widget) _array_element)
      (CallFunction|ObjectiveCompleted)
      (Development|PrintString "Completed"))))

(event Custom|Objective%20Completed
  (for _array_element (.objectives (Variables|Default|GetActiveQuest))
    (if (.Completed (Utilities|Struct|BreakS_QuestObjective _array_element))
      (Math|Integer|IncrementInt (Variables|Default|GetObjectivesCompleted)
        (:%20%20
          (if (>= (Variables|Default|GetObjectivesCompleted) (Utilities|Array|Length (.objectives (Variables|Default|GetActiveQuest))))
            (Development|PrintString "Quest Completed")
            (Variables|Default|SetActiveQuest "")
            (Variables|Default|SetObjectivesCompleted 0)
            (Default|PlayQuestCompletedAnimation (Variables|Default|GetQuest%20HUD%20Widget))))))))

(event EventBeginPlay
  (bind _returnvalue (UserInterface|CreateWidget "/Game/-MyContent/UI/HUD/WB_QuestHUD.WB_QuestHUD_C"))
  (bind _output_get (Variables|Default|SetQuest%20HUD%20Widget _returnvalue))
  (UserInterface|Viewport|AddtoViewport _output_get 0)
  (Default|HideQuestPanel (Variables|Default|GetQuest%20HUD%20Widget)))