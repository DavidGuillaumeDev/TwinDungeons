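; BP_QuestGiver is a quest NPC or object that offers a list of quests to the player.
; A trigger overlap shows an interact prompt widget, which rotates every tick to face the camera.
; Interact toggles a WB_QuestGiver screen filled from the Quests array, switching cursor and input mode.
; The screen receives a reference back to the giver, and CloseWidget reuses the same teardown path.
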(event OnComponentBeginOverlap(TriggerRadius)
  (params (OverlappedComponent :type Primitive%20Component%20Object%20Reference) (OtherActor :type Actor%20Object%20Reference) (OtherComp :type Primitive%20Component%20Object%20Reference) (OtherBodyIndex :type Integer) (bFromSweep :type Boolean) (SweepResult :type Hit%20Result%20Structure%20%28by%20ref%29))
  ;[1 1 1] Interact Appear
  (if (== (Game|GetPlayerCharacter 0) OtherActor)
    (Utilities|Casting|CastToBP_ThirdPersonCharacter OtherActor)
    (Rendering|SetVisibility (Variables|Default|GetInteract%20Widget) true false)))

(event OnComponentEndOverlap(TriggerRadius)
  (params (OverlappedComponent :type Primitive%20Component%20Object%20Reference) (OtherActor :type Actor%20Object%20Reference) (OtherComp :type Primitive%20Component%20Object%20Reference) (OtherBodyIndex :type Integer))
  ;[1 1 1] Interact Appear
  (Utilities|Casting|CastToBP_ThirdPersonCharacter OtherActor)
  (Rendering|SetVisibility (Variables|Default|GetInteract%20Widget) false false))

(event Custom|Close%20Widget
  (bind _returnvalue (Game|GetPlayerController 0))
  ;[1 1 1] Interact
  (Widget|RemovefromParent (Variables|Default|GetQuestsWidget))
  (Variables|Default|SetQuestsWidget 0)
  (Variables|/Script/Engine.PlayerController|SetbShowMouseCursor _returnvalue false)
  (Input|SetInputModeGameOnly _returnvalue false)
  (Variables|Default|SetWidgetActive false))

(event EventTick
  (params (DeltaSeconds :type Float%20%28single-precision%29))
  ;[1 1 1] Interact Visibility
  (Transformation|SetWorldRotation (Variables|Default|GetInteract%20Widget) (Math|Rotator|FindLookatRotation (Transformation|GetWorldLocation (Variables|Default|GetInteract%20Widget)) (Transformation|GetWorldLocation (Variables|/Script/Engine.PlayerCameraManager|GetTransformComponent (Game|GetPlayerCameraManager 0)))) false false))

(event EventInteract
  (bind _returnvalue (Game|GetPlayerController 0))
  (bind _returnvalue_2 (Game|GetPlayerController 0))
  ;[1 1 1] Interact
  (if (not (Variables|Default|GetWidgetActive))
    (bind _returnvalue_3 (UserInterface|CreateWidget "/Game/-MyContent/QuestSystem/WB_QuestGiver.WB_QuestGiver_C"))
    (bind _output_get (Variables|Default|SetQuestsWidget _returnvalue_3))
    (UserInterface|Viewport|AddtoViewport _output_get 0)
    (Variables|Default|SetWidgetActive true)
    (Variables|/Script/Engine.PlayerController|SetbShowMouseCursor _returnvalue_2 true)
    (Input|SetInputModeGameandUI _returnvalue_2 (Variables|Default|GetQuestsWidget) "DoNotLock" true false)
    (Variables|/Game/-MyContent/QuestSystem/WB_QuestGiver.WB_QuestGiver_C|SetQuestGiverBP (Variables|Default|GetQuestsWidget) self)
    (for _array_element (Variables|Default|GetQuests)
      (Default|AddQuest (Variables|Default|GetQuestsWidget) _array_element))
    (else
      (Widget|RemovefromParent (Variables|Default|GetQuestsWidget))
      (Variables|Default|SetQuestsWidget 0)
      (Variables|/Script/Engine.PlayerController|SetbShowMouseCursor _returnvalue false)
      (Input|SetInputModeGameOnly _returnvalue false)
      (Variables|Default|SetWidgetActive false))))

(fn ConstructionScript)