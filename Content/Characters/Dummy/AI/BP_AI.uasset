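; Enemy dummy AI character with a camera-facing health bar and a three-hit sword combo triggered through its Attack function.
; Combo montages chain by attack index and a buffered-attack flag.
; A looping timer runs sphere traces along the sword, applying throttled damage and blood effects to "damage"-tagged actors.
; Taking damage plays a random hit montage, launches it along the player's facing, resets the combo, and ragdolls it when DecreaseHealth returns true.
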(event Custom|Sword%20Attack
  ;[1 1 1] Sword Attack
  ;;[1 1 1] Sword Attack
  (if (Variables|Default|GetisAttacking?)
    (Variables|Default|SetsaveAttack? true)
    (else
      (Variables|Default|SetisAttacking? true)
      (switch int (Variables|Default|GetattackIndex)
        (:0
          (CallFunction|Attack1))
        (:1
          (CallFunction|Attack2))
        (:2
          (CallFunction|Attack3))))))

(event Custom|Sword%20Attack%20Combo
  ;[1 1 1] Sword Attack
  ;;[1 1 1] Combo Continue
  (if (Variables|Default|GetsaveAttack?)
    (Variables|Default|SetsaveAttack? false)
    (switch int (Variables|Default|GetattackIndex)
      (:0
        (CallFunction|Attack1))
      (:1
        (CallFunction|Attack2))
      (:2
        (CallFunction|Attack3)))
    (else
      (CallFunction|StopCombo))))

(event Custom|Start%20Sword%20Trace
  ;[0.05127 0.05127 0.05127] Sword Trace
  (bind _returnvalue (Utilities|Time|SetTimerbyEvent (delegate Custom|Sword%20Trace%20Loop) 0.001 true))
  (Variables|Default|SetswordTraceLoop _returnvalue))

(event Custom|Sword%20Trace%20Loop
  ;[0.05127 0.05127 0.05127] Sword Trace
  (bind (_outhit _returnvalue) (Collision|SphereTraceByChannel (Transformation|GetWorldLocation (Variables|Default|GetSword_Top_Point)) (Transformation|GetWorldLocation (Variables|Default|GetSword_Bottom_Point)) 12.0 "TraceTypeQuery1" false 0 "ForDuration" true "(R=1.000000,G=0.000000,B=0.000000,A=1.000000)" "(R=0.000000,G=1.000000,B=0.000000,A=1.000000)" 0.2))
  (if _returnvalue
    (if (Actor|ActorHasTag (.HitActor (Collision|BreakHitResult _outhit)) "damage")
      (Utilities|FlowControl|DoOnce false :!label _label
        (:Completed
          (Game|Damage|ApplyDamage (.HitActor (Collision|BreakHitResult _outhit)) 1e+01 0 0)
          (Effects|SpawnEmitteratLocation "/Game/FX/Particles/Blood/P_Blood_Splat_Cone.P_Blood_Splat_Cone" (.Location (Collision|BreakHitResult _outhit)) (Math|Rotator|MakeRotfromXY (.Normal (Collision|BreakHitResult _outhit)) (.Normal (Collision|BreakHitResult _outhit))) "0.400000,0.400000,0.400000" true "AutoRelease")
          (Utilities|FlowControl|Delay 0.5)
          (goto _label Reset))))))

(event Custom|Stop%20Sword%20Trace
  ;[0.05127 0.05127 0.05127] Sword Trace
  (Utilities|Time|ClearandInvalidateTimerbyHandle (Variables|Default|GetswordTraceLoop)))

(event Custom|Stop%20Combo
  ;[1 1 1] Sword Attack
  ;;[1 1 1] Stop Combo/Attack
  (Variables|Default|SetisAttacking? false)
  (Variables|Default|SetattackIndex 0))

(event Custom|Ragdoll
  ;[1 1 1] Ragdoll
  (Utilities|FlowControl|Delay 2.5)
  (Physics|SetSimulatePhysics (Variables|Character|GetMesh) true))

(event Custom|Attack%201
  ;[1 1 1] Sword Attack
  ;;[1 1 1] Attack 1
  (Utilities|FlowControl|DoOnce false :!label _label
    (:Completed
      (Utilities|FlowControl|Delay 0.1)
      (Animation|Montage|PlayMontage (Variables|Character|GetMesh) "/Game/Characters/RPG_Character/Animations/SwordAttacks/Montage/Attack1_Montage.Attack1_Montage"
        (:then
          (Variables|Default|SetattackIndex 1)
          (goto _label Reset))))))

(event Custom|Sword%20Attack%20Combo%20Call%20From%20BT
  ;[1 1 1] Sword Attack
  ;;[1 1 1] Attack Input
  (if (Variables|Default|GetcanAttack?)
    (CallFunction|SwordAttack)))

(event Custom|Attack%202
  ;[1 1 1] Sword Attack
  ;;[1 1 1] Attack 2
  (Utilities|FlowControl|DoOnce false :!label _label
    (:Completed
      (Utilities|FlowControl|Delay 0.1)
      (Animation|Montage|PlayMontage (Variables|Character|GetMesh) "/Game/Characters/RPG_Character/Animations/SwordAttacks/Montage/Attack2_Montage.Attack2_Montage"
        (:then
          (Variables|Default|SetattackIndex 2)
          (goto _label Reset))))))

(event Custom|Attack%203
  ;[1 1 1] Sword Attack
  ;;[1 1 1] Attack 3
  (Utilities|FlowControl|DoOnce false :!label _label
    (:Completed
      (Utilities|FlowControl|Delay 0.1)
      (Animation|Montage|PlayMontage (Variables|Character|GetMesh) "/Game/Characters/RPG_Character/Animations/SwordAttacks/Montage/Attack3_Montage.Attack3_Montage"
        (:then
          (Variables|Default|SetattackIndex 3)
          (goto _label Reset))))))

(event Game|Damage|EventAnyDamage
  (params (Damage :type Float%20%28single-precision%29) (DamageType :type Damage%20Type%20Object%20Reference) (InstigatedBy :type Controller%20Object%20Reference) (DamageCauser :type Actor%20Object%20Reference))
  ;[1 1 1] Take Damage
  (Utilities|FlowControl|Sequence
    (:then_0
      (Animation|PlayAnimMontage (Utilities|Array|Get(acopy) (Variables|Default|GetHit%20Anims) (Math|Random|RandomIntegerinRange 0 (- (Utilities|Array|Length (Variables|Default|GetHit%20Anims)) 1))) 1.0 "None")
      (bind _asbp_third_person_character (Utilities|Casting|CastToBP_ThirdPersonCharacter (Game|GetPlayerCharacter 0)))
      (Character|LaunchCharacter (* (Math|Vector|GetForwardVector (Transformation|GetActorRotation _asbp_third_person_character)) 7e+02) false false)
      (bind _is_player_dead_ (Default|DecreaseHealth (Variables|Default|GetAC_Player_Stats) Damage))
      (if _is_player_dead_
        (Collision|SetCollisionObjectType (Variables|Character|GetMesh) "ECC_PhysicsBody")
        (Utilities|FlowControl|Sequence
          (:then_0
            (Physics|SetSimulatePhysics (Variables|Character|GetMesh) true))
          (:then_1
            (Development|SetHiddeninGame (Variables|Default|GetHealth%20Bar%20Widget) true false))
          (:then_2
            (Collision|SetCollisionEnabled (Variables|Collision|GetCapsuleComponent) "NoCollision")))))
    (:then_2
      (CallFunction|StopCombo))))

(event EventTick
  (params (DeltaSeconds :type Float%20%28single-precision%29))
  ;[1 1 1] Widget HP
  (Transformation|SetWorldRotation (Variables|Default|GetHealth%20Bar%20Widget) (Math|Rotator|FindLookatRotation (Transformation|GetWorldLocation (Variables|Character|GetMesh)) (Transformation|GetWorldLocation (Variables|/Script/Engine.PlayerCameraManager|GetTransformComponent (Game|GetPlayerCameraManager 0)))) false false))

(event EventBeginPlay
  ;[1 1 1] Widget HP
  (bind _aswb_dummy_health_bar (Utilities|Casting|CastToWB_DummyHealthBar (UserInterface|GetWidget (Variables|Default|GetHealth%20Bar%20Widget))))
  (Variables|Default|Sethealth_bar_ui _aswb_dummy_health_bar))

(fn ConstructionScript)

(fn Attack
  (CallFunction|SwordAttackComboCallfromBT)
  (return 0.4))